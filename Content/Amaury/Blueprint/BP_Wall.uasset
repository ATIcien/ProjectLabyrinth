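; BP_Wall is a wall actor that starts moving and triggers a dolly zoom on the player when they enter its trigger box.
; It caches the third-person character on BeginPlay, then on overlap with an actor tagged "Player" activates its InterpToMovement component and calls the character's EventDollyZoom.
; The trigger box then switches to NoCollision so the sequence fires only once.
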(event `self.ReceiveBeginPlay`
  (bind _asbp_third_person_character (cast `/Game/ThirdPerson/Blueprints/BP_ThirdPersonCharacter` (`GameplayStatics.GetPlayerCharacter` 0)))
  (set `self.As BP Third Person Character` _asbp_third_person_character))

(event `self.TriggerBox.OnComponentBeginOverlap`
  (params (OverlappedComponent :type "PrimitiveComponent Object Reference") (OtherActor :type "Actor Object Reference") (OtherComp :type "PrimitiveComponent Object Reference") (OtherBodyIndex :type Integer) (bFromSweep :type Boolean) (SweepResult :type "HitResult Structure (by ref)"))
  (if (`self.ActorHasTag` OtherActor "Player")
    (`ActorComponent.Activate` (`self.InterpToMovement`) false)
    (`/Game/ThirdPerson/Blueprints/BP_ThirdPersonCharacter.Event_DollyZoom` (`self.As BP Third Person Character`))
    (`PrimitiveComponent.SetCollisionProfileName` (`self.TriggerBox`) "NoCollision" true)))

(fn `UserConstructionScript`)