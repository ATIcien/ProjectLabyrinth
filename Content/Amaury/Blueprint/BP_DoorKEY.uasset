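; BP_DoorKEY is a key-locked door that the player opens and closes through an Interact event while its button prompt is visible.
; A box overlap shows or hides the prompt widget created on BeginPlay, and that visibility gates interaction.
; The first opening takes a key from the player and leaves the door unlocked afterward.
; A timeline rotates the pivot's yaw a quarter turn, with RevertRotation choosing the direction, and reverses to close.
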(event `self.ReceiveBeginPlay`
  ;[1 1 1] Widget
  (bind _returnvalue (`|CreateWidget` "/Game/Amaury/Blueprint/Widget_Button.Widget_Button_C"))
  (bind _output_get (set `self.Button_Wid` _returnvalue))
  (`UserWidget.AddToViewport` _output_get 0)
  (set `self.IsDoorUnlocked` false))

(event `self.Box.OnComponentBeginOverlap`
  (params (OverlappedComponent :type "PrimitiveComponent Object Reference") (OtherActor :type "Actor Object Reference") (OtherComp :type "PrimitiveComponent Object Reference") (OtherBodyIndex :type Integer) (bFromSweep :type Boolean) (SweepResult :type "HitResult Structure (by ref)"))
  ;[1 1 1] ButtonVisibilty
  (`Widget.SetVisibility` (`self.Button_Wid`) "Visible"))

(event `self.Box.OnComponentEndOverlap`
  (params (OverlappedComponent :type "PrimitiveComponent Object Reference") (OtherActor :type "Actor Object Reference") (OtherComp :type "PrimitiveComponent Object Reference") (OtherBodyIndex :type Integer))
  ;[1 1 1] ButtonVisibilty
  (`Widget.SetVisibility` (`self.Button_Wid`) "Hidden"))

(event `/Game/Amaury/Blueprint/Bp_Interface_Intreract.Interact`
  (params (Player :type "/Game/ThirdPerson/Blueprints/BP_ThirdPersonCharacter Object Reference"))
  ;[1 1 1] Interact
  (if (`Widget.IsVisible` (`self.Button_Wid`))
    (if (not (`self.IsdoorOpen`))
      (if (`self.IsDoorUnlocked`)
        (set `self.IsdoorOpen` true :!label _label)
        (bind (_direction _dooropen_time) (`Timeline|Timeline` :!label _label_2)
          (:`Update`
            (`SceneComponent.K2_SetRelativeRotation` (`self.DoorPivot`) (`KismetMathLibrary.MakeRotator` 0.0 0.0 (`KismetMathLibrary.Lerp` 0.0 (`KismetMathLibrary.SelectFloat` -90.0 90.0 (`self.RevertRotation`)) _dooropen_time)) false false)))
        (else
          (bind _success (`/Game/ThirdPerson/Blueprints/BP_ThirdPersonCharacter.RemoveKey` Player))
          (if _success
            (set `self.IsDoorUnlocked` true)
            (goto _label))))
      (else
        (set `self.IsdoorOpen` false)
        (goto _label_2 :!via `Reverse`)))))

(fn `UserConstructionScript`)