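; BP_Invisible is an actor that drives a location-based dissolve material and reacts to the player entering its trigger.
; Every tick it writes its static mesh's world location and scale into a dissolve Material Parameter Collection.
; A tagged Player overlapping TriggerBox activates the InterpToMovement component and fires a collision event dispatcher.
; The player character reference cached on BeginPlay is unused here, and CountDownTrigger is empty.
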(event `self.ReceiveTick`
  (params (DeltaSeconds :type "Float (single-precision)"))
  (bind _staticmeshcomponent (`self.StaticMeshComponent`))
  ;[1 1 1] Mat_Parameter
  (`KismetMaterialLibrary.SetVectorParameterValue` "/Game/Amaury/Mat/MAT_Paraneter_Disolve.MAT_Paraneter_Disolve" "Location" (`KismetMathLibrary.Conv_VectorToLinearColor` (`SceneComponent.K2_GetComponentLocation` _staticmeshcomponent)))
  (`KismetMaterialLibrary.SetVectorParameterValue` "/Game/Amaury/Mat/MAT_Paraneter_Disolve.MAT_Paraneter_Disolve" "Scale" (`KismetMathLibrary.Conv_VectorToLinearColor` (`SceneComponent.K2_GetComponentScale` _staticmeshcomponent))))

(event `self.ReceiveBeginPlay`
  ;[1 1 1] Charactere
  (bind _asbp_third_person_character (cast `/Game/ThirdPerson/Blueprints/BP_ThirdPersonCharacter` (`GameplayStatics.GetPlayerCharacter` 0)))
  (set `self.As BP Third Person Character` _asbp_third_person_character))

(event `self.TriggerBox.OnComponentBeginOverlap`
  (params (OverlappedComponent :type "PrimitiveComponent Object Reference") (OtherActor :type "Actor Object Reference") (OtherComp :type "PrimitiveComponent Object Reference") (OtherBodyIndex :type Integer) (bFromSweep :type Boolean) (SweepResult :type "HitResult Structure (by ref)"))
  ;[1 1 1] Trigger
  (if (`self.ActorHasTag` OtherActor "Player")
    (`ActorComponent.Activate` (`self.InterpToMovement`) false)
    (`self.OnCollisonEventDispa`)))

(fn `CountDownTrigger`)

(fn `UserConstructionScript`)