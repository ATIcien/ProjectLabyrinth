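; BP_LightTrigger is a trigger actor that lights up an array of fire lights when any actor overlaps it.
; BeginPlay starts each referenced light off by zeroing its LightFire intensity and hiding its Flamme component.
; Begin overlap sets LightFire to the Intensity variable and shows Flamme.
; The lights stay on afterwards, as the switch-off loop is not connected to EndOverlap or any other event.
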(event `self.ReceiveBeginPlay`
  (for _array_element (`self.Light`)
    (`LightComponent.SetIntensity` (`/Game/Amaury/Blueprint/BP_Light.LightFire` _array_element) 0.0)
    (`SceneComponent.SetVisibility` (`/Game/Amaury/Blueprint/BP_Light.Flamme` _array_element) false false)))

(event `self.ReceiveActorBeginOverlap`
  (params (OtherActor :type "Actor Object Reference"))
  (for _array_element (`self.Light`)
    (`LightComponent.SetIntensity` (`/Game/Amaury/Blueprint/BP_Light.LightFire` _array_element) (`self.Intensity`))
    (`SceneComponent.SetVisibility` (`/Game/Amaury/Blueprint/BP_Light.Flamme` _array_element) true false)))

(event `self.ReceiveActorEndOverlap`
  (params (OtherActor :type "Actor Object Reference")))

(fn `UserConstructionScript`)