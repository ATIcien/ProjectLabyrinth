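; Interactable torch switch that opens and closes a linked door, with an on-screen button prompt.
; Entering the trigger box shows the prompt widget and lights the child BP_Light's fire and flame, which stay lit after the player leaves.
; Interact works only while the prompt is visible, using a FlipFlop to play or reverse a timeline that raises the door mesh and tilts the torch like a lever.
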(event `self.ReceiveBeginPlay`
  (bind _returnvalue (`|CreateWidget` "/Game/Amaury/Blueprint/Widget_Button.Widget_Button_C"))
  (bind _output_get (set `self.Button Ref` _returnvalue))
  (`UserWidget.AddToViewport` _output_get 0)
  (bind _asbp_light (cast `/Game/Amaury/Blueprint/BP_Light` (`ChildActorComponent.ChildActor` (`self.ChildActor_Light`))))
  (set `self.Light` _asbp_light)
  (`LightComponent.SetIntensity` (`/Game/Amaury/Blueprint/BP_Light.LightFire` (`self.Light`)) 0.0)
  (`SceneComponent.SetVisibility` (`/Game/Amaury/Blueprint/BP_Light.Flamme` (`self.Light`)) false false))

(event `self.Box1.OnComponentBeginOverlap`
  (params (OverlappedComponent :type "PrimitiveComponent Object Reference") (OtherActor :type "Actor Object Reference") (OtherComp :type "PrimitiveComponent Object Reference") (OtherBodyIndex :type Integer) (bFromSweep :type Boolean) (SweepResult :type "HitResult Structure (by ref)"))
  (`Widget.SetVisibility` (`self.Button Ref`) "Visible")
  (`LightComponent.SetIntensity` (`/Game/Amaury/Blueprint/BP_Light.LightFire` (`self.Light`)) (`self.Intensity`))
  (`SceneComponent.SetVisibility` (`/Game/Amaury/Blueprint/BP_Light.Flamme` (`self.Light`)) true false))

(event `self.Box1.OnComponentEndOverlap`
  (params (OverlappedComponent :type "PrimitiveComponent Object Reference") (OtherActor :type "Actor Object Reference") (OtherComp :type "PrimitiveComponent Object Reference") (OtherBodyIndex :type Integer))
  (`Widget.SetVisibility` (`self.Button Ref`) "Hidden"))

(event `/Game/Amaury/Blueprint/Bp_Interface_Intreract.Interact`
  (params (Player :type "/Game/ThirdPerson/Blueprints/BP_ThirdPersonCharacter Object Reference"))
  (if (`Widget.IsVisible` (`self.Button Ref`))
    (`/Engine/EditorBlueprintResources/StandardMacros.FlipFlop`
      (:`A`
        (bind (_direction _floatvalue) (`Timeline|Timeline` :!label _label)
          (:`Update`
            (`SceneComponent.K2_SetRelativeLocation` (`/Game/Amaury/Blueprint/BP_Door.Door_Mesh` (`self.DoorOpen_BP`)) (`KismetMathLibrary.MakeVector` 0.0 0.0 (`KismetMathLibrary.Lerp` 0.0 410.0 _floatvalue)) false false)
            (`SceneComponent.K2_SetRelativeRotation` (`self.ChildActor_Light`) (`KismetMathLibrary.MakeRotator` (`KismetMathLibrary.Lerp` 0.0 -13.0 _floatvalue)) false false)
            (`KismetSystemLibrary.PrintString` "Test1"))))
      (:`B`
        (goto _label :!via `Reverse`)))))

(fn `UserConstructionScript`)